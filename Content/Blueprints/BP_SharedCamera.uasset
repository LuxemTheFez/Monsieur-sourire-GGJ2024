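; BP_SharedCamera is a shared camera that frames two players, following their midpoint and zooming with their separation.
; Tick looks up both player characters until valid, then updates distance, center point, zoom and positions.
; Spring arm length eases toward half the offset-adjusted player distance using FInterpTo.
; The Box moves to the X-offset midpoint, while the spring arm's world position follows it only along Y.
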(event EventTick
  (params (DeltaSeconds :type Float%20%28single-precision%29))
  (if (and (Utilities|IsValid (Variables|Default|Getplayer1)) (Utilities|IsValid (Variables|Default|Getplayer2)))
    (Variables|Default|SetDelta DeltaSeconds)
    (CallFunction|GetPlayerDistance)
    (CallFunction|GetCenterPoint)
    (CallFunction|Zoom)
    (CallFunction|SetBoxPosition)
    (else
      (Variables|Default|Setplayer1 (Game|GetPlayerCharacter 0))
      (Variables|Default|Setplayer2 (Game|GetPlayerCharacter 1)))))

(fn ConstructionScript)

(fn GetPlayerDistance
  (Variables|Default|SetplayerDistance (- (Transformation|GetDistanceTo (Variables|Default|Getplayer1) (Variables|Default|Getplayer2)) 2e+02)))

(fn GetCenterPoint
  (bind _player1 (Variables|Default|Getplayer1))
  (bind _player2 (Variables|Default|Getplayer2))
  (bind _returnvalue (Transformation|GetActorLocation _player2))
  (bind _returnvalue_2 (Transformation|GetActorLocation _player1))
  (bind _returnvalue_3 (+ _returnvalue_2 _returnvalue))
  (bind _returnvalue_4 (/ _returnvalue_3 2.0))
  (Variables|Default|SetCenterPoint (Math|Vector|MakeVector (- (.x _returnvalue_4) (Variables|Default|GetcameraOffset)) (.y _returnvalue_4) (.z _returnvalue_4))))

(fn Zoom
  (bind _springarm (Variables|Default|GetSpringArm))
  (Variables|/Script/Engine.SpringArmComponent|SetTargetArmLength _springarm (Math|Interpolation|FInterpTo (Variables|/Script/Engine.SpringArmComponent|GetTargetArmLength _springarm) (/ (Variables|Default|GetplayerDistance) 2.0) (Variables|Default|GetDelta) 1.0)))

(fn SetBoxPosition
  (bind _springarm (Variables|Default|GetSpringArm))
  (bind _returnvalue (Transformation|GetWorldLocation _springarm))
  (Transformation|SetWorldLocation (Variables|Default|GetBox) (Variables|Default|GetCenterPoint) false false)
  (Transformation|SetWorldLocation _springarm (Math|Vector|MakeVector (.x _returnvalue) (.y (Variables|Default|GetCenterPoint)) (.z _returnvalue)) false false))