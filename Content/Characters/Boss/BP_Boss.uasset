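; Boss character whose amusement meter decays each second and sets one of four moods, taking damage only in the top, laughing mood.
; Entertain calls add fun scaled by per-entertainer-class modifiers, then mood updates from thresholds, also refreshed every Tick.
; ConsiderEntertainer aims to penalize repeated entertainers and favor others, but edits copies of map values without writing back.
; Die is an empty stub.
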(event EventBeginPlay
  (Components|Animation|PlayAnimation (Variables|Default|GetSkeletalMesh) "/Game/Characters/Boss/A_Boss_Idle_Sequence.A_Boss_Idle_Sequence" true))

(event Collision|EventActorBeginOverlap
  (params (OtherActor :type Actor%20Object%20Reference)))

(event EventTick
  (params (DeltaSeconds :type Float%20%28single-precision%29))
  (Variables|Default|SetTimeSinceLastLoseAmusement (+ DeltaSeconds (Variables|Default|GetTimeSinceLastLoseAmusement)))
  (while (>= (Variables|Default|GetTimeSinceLastLoseAmusement) 1.0)
    (CallFunction|LoseAmusement)
    (Math|Float|DecrementFloat (Variables|Default|GetTimeSinceLastLoseAmusement)))
  (CallFunction|UpdateMood))

(fn ConstructionScript)

(fn IsVulnerable
  (return (>= (Variables|Default|GetAmusementMetter) 1.0)))

(fn LoseAmusement
  (Variables|Default|SetAmusementMetter (- (Variables|Default|GetAmusementMetter) 0.01)))

(fn UpdateMood
  (Development|PrintString (Utilities|String|ToString(Float) (Variables|Default|GetAmusementMetter)))
  (bind _output_get (Variables|Default|SetAmusementMetter (Math|Float|Max(Float) (Variables|Default|GetAmusementMetter) 0.0)))
  (if (< _output_get (Variables|Default|GetNeutralMoodThreshold))
    (Variables|Default|SetCurrentMood "NewEnumerator0")
    (elif (< _output_get (Variables|Default|GetSmilingMoodThreshold))
      (Variables|Default|SetCurrentMood "NewEnumerator1")
      (elif (< _output_get (Variables|Default|GetLaughingMoodThreshold))
        (Variables|Default|SetCurrentMood "NewEnumerator2")
        (else
          (Variables|Default|SetCurrentMood "NewEnumerator3")
          (Components|Animation|PlayAnimation (Variables|Default|GetSkeletalMesh) "/Game/Characters/Boss/A_Boss_Laugh_Sequence.A_Boss_Laugh_Sequence" true))))))

(fn GetAttacked
  (params (IncomingDamage :type Integer))
  (if (Utilities|Enum|Equal(Enum) (Variables|Default|GetCurrentMood) "NewEnumerator3")
    (Default|TakeDamage (Variables|Default|GetHealth) IncomingDamage)
    (if (<= (Variables|/Game/Characters/BP_HealthSystem_AC.BP_HealthSystem_AC_C|GetcurentHealth (Variables|Default|GetHealth)) 0)
      (CallFunction|Die))))

(fn Die)

(fn Entertain
  (params (FunAddedPercent :type Float%20%28double-precision%29) (EntertainerClass :type BP%20Item%20Class%20Reference))
  (bind _modifiersmap (Variables|Default|GetModifiersMap))
  (bind (_value _returnvalue) (Utilities|Map|Find _modifiersmap EntertainerClass))
  (if _returnvalue
    (Variables|Default|SetAmusementMetter (+ (* _value FunAddedPercent) (Variables|Default|GetAmusementMetter)))
    (CallFunction|UpdateMood)
    (CallFunction|ConsiderEntertainer EntertainerClass)))

(fn EntertainOverTime
  (params (FunAddedPercent :type Float%20%28double-precision%29) (EntertainerClass :type BP%20Item%20Class%20Reference))
  (bind _modifiersmap (Variables|Default|GetModifiersMap))
  (bind (_value _returnvalue) (Utilities|Map|Find _modifiersmap EntertainerClass))
  (if _returnvalue
    (Variables|Default|SetAmusementMetter (+ (* _value FunAddedPercent) (Variables|Default|GetAmusementMetter)))
    (CallFunction|UpdateMood)))

(fn ConsiderEntertainer
  (params (entertainer :type BP%20Item%20Class%20Reference))
  (bind _keys (Utilities|Map|Keys (Variables|Default|GetModifiersMap)))
  (for (_array_element _array_index) _keys
    (if (== _array_element entertainer)
      (bind _values (Utilities|Map|Values (Variables|Default|GetModifiersMap)))
      (Utilities|Array|SetArrayElem _values _array_index (Math|Float|Max(Float) (- (Utilities|Array|Get(acopy) _values _array_index) 0.15) 0.0))
      (else
        (bind _values_2 (Utilities|Map|Values (Variables|Default|GetModifiersMap)))
        (Utilities|Array|SetArrayElem _values_2 _array_index (+ (Utilities|Array|Get(acopy) _values_2 _array_index) 0.05))))))