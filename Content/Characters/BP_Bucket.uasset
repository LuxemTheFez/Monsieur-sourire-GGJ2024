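; BP_Bucket is a bucket that visually shows how full of poop it is.
; Every Tick, it places the Poop component by lerping between the relative transforms of PoopBaseTransform and PoopFilledTransform, using FillPercent as alpha.
; PoopOverflow and its children stay hidden in game until FillPercent reaches 1.
; The Blueprint only reads FillPercent and never changes it.
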(event EventBeginPlay)

(event EventTick
  (params (DeltaSeconds :type Float%20%28single-precision%29))
  (Transformation|SetRelativeTransform (Variables|Default|GetPoop) (Math|Transform|Lerp(Transform) (Transformation|GetRelativeTransform (Variables|Default|GetPoopBaseTransform)) (Transformation|GetRelativeTransform (Variables|Default|GetPoopFilledTransform)) (Variables|Default|GetfillPercent)) false true)
  (Development|SetHiddeninGame (Variables|Default|GetPoopOverflow) (< (Variables|Default|GetfillPercent) 1.0) true))

(fn ConstructionScript)