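; BP_Spawner is an enemy spawner that spawns escalating waves of monsters around itself.
; A looping timer started on BeginPlay runs SpawnMonsters in a loop sized by SpawnNumber.
; Each call spawns one light and one heavy enemy at random reachable navmesh points within a radius.
; HandleSpawn counts these pairs, raising SpawnNumber and resetting the count at a threshold that grows with SpawnNumber, so each escalation needs more pairs.
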(event Custom|Spawn
  ;[1 1 1] While loop for enemy spawn
  (for _index (range 0 (Variables|Default|GetSpawnNumber))
    (CallFunction|SpawnMonsters)))

(event Custom|SpawnMonsters
  (bind _returnvalue (Transformation|GetActorLocation))
  ;[1 1 1] Spawn 2 monsters, one big and one little
  (Game|SpawnActorfromClass "/Game/Characters/Enemies/BP_Light_Enemy.BP_Light_Enemy_C" (Math|Conversions|ToTransform(Vector) (.RandomLocation (AI|Navigation|GetRandomReachablePointinRadius _returnvalue 2e+03 0 0))) "Undefined" "MultiplyWithRoot" 0 0)
  (Game|SpawnActorfromClass "/Game/Characters/Enemies/BP_Heavy_Enemy.BP_Heavy_Enemy_C" (Math|Conversions|ToTransform(Vector) (.RandomLocation (AI|Navigation|GetRandomReachablePointinRadius _returnvalue 2e+03 0 0))) "Undefined" "MultiplyWithRoot" 0 0)
  (CallFunction|HandleSpawn))

(event Custom|HandleSpawn
  ;[1 1 1] Handle Spawn (increase amount spawn and time between increasing amount spawn)
  (bind _result (Math|Integer|IncrementInt (Variables|Default|GetSpawnCount))
    (:%20%20
      (bind _output_get (Variables|Default|SetSpawnCount _result))
      (if (>= _output_get (+ (* (Variables|Default|GetSpawnNumber) 5) 5))
        (Variables|Default|SetSpawnCount 0)
        (bind _result_2 (Math|Integer|IncrementInt (Variables|Default|GetSpawnNumber))
          (:%20%20
            (Variables|Default|SetSpawnNumber _result_2)))))))

(event EventBeginPlay
  ;[1 1 1] While loop for enemy spawn
  (Variables|Default|SetSpawnNumber 0)
  (Utilities|Time|SetTimerbyEvent (delegate Custom|Spawn) 7.5 true))

(fn ConstructionScript)