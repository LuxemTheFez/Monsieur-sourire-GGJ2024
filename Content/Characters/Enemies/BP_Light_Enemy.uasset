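; BP_Light_Enemy is an enemy character that chases the player and can be killed.
; It starts at MaxHealth and runs AIMoveTo toward the player character, re-issuing the move only on success.
; AnyDamage lowers clamped health; at zero, Death plays a jump animation, disables movement and destroys the actor after a short delay.
; HitRange overlaps toggle an InRange flag without filtering the actor, and no attack logic uses it here.
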(event OnComponentBeginOverlap(HitRange)
  (params (OverlappedComponent :type Primitive%20Component%20Object%20Reference) (OtherActor :type Actor%20Object%20Reference) (OtherComp :type Primitive%20Component%20Object%20Reference) (OtherBodyIndex :type Integer) (bFromSweep :type Boolean) (SweepResult :type Hit%20Result%20Structure%20%28by%20ref%29))
  ;[1 1 1] Hitting Player
  (Variables|Default|SetInRange true))

(event OnComponentEndOverlap(HitRange)
  (params (OverlappedComponent :type Primitive%20Component%20Object%20Reference) (OtherActor :type Actor%20Object%20Reference) (OtherComp :type Primitive%20Component%20Object%20Reference) (OtherBodyIndex :type Integer))
  ;[1 1 1] Hitting Player
  (Variables|Default|SetInRange false))

(event Custom|FollowPlayer
  ;[1 1 1] Base behavior
  (AI|AIMoveTo self "0, 0, 0" (Game|GetPlayerCharacter 0) 5.0 false
    (:OnSuccess
      (CallFunction|FollowPlayer))))

(event Custom|Death
  (bind _charactermovement (Variables|Character|GetCharacterMovement))
  ;[1 1 1] Dying
  (Variables|Default|SetDead true)
  (Components|Animation|PlayAnimation (Variables|Character|GetMesh) "/Game/Characters/Mannequins/Animations/Manny/MM_Jump.MM_Jump" false)
  (Components|Movement|StopMovementImmediately _charactermovement)
  (Pawn|Components|CharacterMovement|DisableMovement _charactermovement)
  (Utilities|FlowControl|Delay 1.0)
  (Actor|DestroyActor))

(event EventBeginPlay
  ;[1 1 1] Base behavior
  (Variables|Default|SetCurrentHealth (Variables|Default|GetMaxHealth))
  (CallFunction|FollowPlayer))

(event Game|Damage|EventAnyDamage
  (params (Damage :type Float%20%28single-precision%29) (DamageType :type Damage%20Type%20Object%20Reference) (InstigatedBy :type Controller%20Object%20Reference) (DamageCauser :type Actor%20Object%20Reference))
  ;[1 1 1] Taking Damage
  (if (not (Variables|Default|GetDead))
    (Variables|Default|SetCurrentHealth (Math|Float|Clamp(Float) (- (Variables|Default|GetCurrentHealth) Damage) 0.0 (Variables|Default|GetMaxHealth)))
    (if (== (Variables|Default|GetCurrentHealth) 0.0)
      (CallFunction|Death))))

(fn ConstructionScript)