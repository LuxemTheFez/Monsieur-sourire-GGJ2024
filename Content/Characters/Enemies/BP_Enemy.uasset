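; Enemy character that chases the player, damages them on contact and may drop a random item when killed.
; BeginPlay picks a random color material and starts an AI MoveTo that reissues itself on each success.
; While HitRange is overlapped, Tick sphere-tests for the player and damages their health component, using a Hitting flag to hit once per contact.
; Incoming damage has a short cooldown, and death plays an animation before the drop roll and destruction.
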(event OnComponentBeginOverlap(HitRange)
  (params (OverlappedComponent :type Primitive%20Component%20Object%20Reference) (OtherActor :type Actor%20Object%20Reference) (OtherComp :type Primitive%20Component%20Object%20Reference) (OtherBodyIndex :type Integer) (bFromSweep :type Boolean) (SweepResult :type Hit%20Result%20Structure%20%28by%20ref%29))
  ;[1 1 1] Hitting Player
  (Variables|Default|SetInRange true))

(event OnComponentEndOverlap(HitRange)
  (params (OverlappedComponent :type Primitive%20Component%20Object%20Reference) (OtherActor :type Actor%20Object%20Reference) (OtherComp :type Primitive%20Component%20Object%20Reference) (OtherBodyIndex :type Integer))
  ;[1 1 1] Hitting Player
  (Variables|Default|SetInRange false))

(event Custom|FollowPlayer
  ;[1 1 1] Base behavior
  (AI|AIMoveTo self "0, 0, 0" (Game|GetPlayerCharacter 0) 5.0 false
    (:OnSuccess
      (CallFunction|FollowPlayer))))

(event Custom|Set%20Material
  (bind _mesh (Variables|Character|GetMesh))
  ;[1 1 1] Set Color Mesh
  (if (== (Variables|Default|GetColor) 0)
    (Rendering|Material|SetMaterial _mesh 0 "/Game/Characters/Enemies/M_Ennemi_Blue.M_Ennemi_Blue")
    (elif (== (Variables|Default|GetColor) 1)
      (Rendering|Material|SetMaterial _mesh 0 "/Game/Characters/Enemies/M_Ennemi_Yellow.M_Ennemi_Yellow")
      (else
        (Rendering|Material|SetMaterial _mesh 0 "/Game/Characters/Enemies/M_Ennemi_Green.M_Ennemi_Green")))))

(event Custom|Death
  (bind _charactermovement (Variables|Character|GetCharacterMovement))
  ;[1 1 1] Dying
  (Variables|Default|SetDead true)
  (Components|Animation|PlayAnimation (Variables|Character|GetMesh) "/Game/Characters/Mannequins/Animations/Manny/MM_Jump.MM_Jump" false)
  (Components|Movement|StopMovementImmediately _charactermovement)
  (Pawn|Components|CharacterMovement|DisableMovement _charactermovement)
  (Utilities|FlowControl|Delay 1.0)
  (if (<= (Math|Random|RandomFloat) (Variables|Default|GetdropChance))
    (CallFunction|DropItem))
  (Actor|DestroyActor))

(event Custom|Drop%20Item
  (bind _returnvalue (Transformation|GetActorTransform))
  ;[1 1 1] Drop item event
  (Game|SpawnActorfromClass (.OutItem (Utilities|Array|Random (Variables|Default|GetpossibleDrops))) (Math|Transform|MakeTransform (Transformation|GetWorldLocation (Variables|Character|GetMesh)) (.rotation _returnvalue) (.scale _returnvalue)) "Undefined" "MultiplyWithRoot" 0 0))

(event Custom|TakeDamage
  (params (Damage :type Float%20%28double-precision%29))
  ;[1 1 1] Taking Damage
  (if (>= (Variables|Default|GetsecondSinceLastDmg) 0.5)
    (Development|PrintString (Utilities|String|ToString(Float) Damage))
    (if (not (Variables|Default|GetDead))
      (Variables|Default|SetCurrentHealth (Math|Float|Clamp(Float) (- (Variables|Default|GetCurrentHealth) Damage) 0.0 (Variables|Default|GetMaxHealth)))
      (Variables|Default|SetsecondSinceLastDmg 0.0)
      (if (<= (Variables|Default|GetCurrentHealth) 0.0)
        (CallFunction|Death)))))

(event EventBeginPlay
  ;[1 1 1] Base behavior
  (Variables|Default|SetBaseDamage 5.0)
  (Variables|Default|SetCurrentHealth (Variables|Default|GetMaxHealth))
  (Variables|Default|SetColor (Utilities|Enum|ByteToEnumColor (Math|Conversions|ToByte(Integer) (Math|Random|RandomIntegerinRange 0 2))))
  (CallFunction|SetMaterial)
  (CallFunction|FollowPlayer))

(event EventTick
  (params (DeltaSeconds :type Float%20%28single-precision%29))
  (bind _hitsphere (Variables|Default|GetHitSphere))
  ;[1 1 1] Hitting Player
  (Variables|Default|SetsecondSinceLastDmg (+ DeltaSeconds (Variables|Default|GetsecondSinceLastDmg)))
  (if (Variables|Default|GetInRange)
    (bind (_outactors _returnvalue) (Collision|SphereOverlapActors (Transformation|GetWorldLocation _hitsphere) (Components|Sphere|GetScaledSphereRadius _hitsphere) (Utilities|Array|MakeArray "ObjectTypeQuery3") "/Game/Characters/BP_PlayerWithAnim.BP_PlayerWithAnim_C"))
    (if (Variables|Default|GetHitting)
      (if (not _returnvalue)
        (Variables|Default|SetHitting false))
      (else
        (for _array_element _outactors
          (bind _asbp_player_with_anim (Utilities|Casting|CastToBP_PlayerWithAnim _array_element))
          (Default|TakeDamage (Variables|/Game/Characters/BP_PlayerWithAnim.BP_PlayerWithAnim_C|GetBP_HealthSystem_AC _asbp_player_with_anim) (Math|Float|Truncate (Variables|Default|GetBaseDamage)))
          (Development|PrintString (Utilities|String|ToString(Integer) (Variables|/Game/Characters/BP_HealthSystem_AC.BP_HealthSystem_AC_C|GetcurentHealth (Variables|/Game/Characters/BP_PlayerWithAnim.BP_PlayerWithAnim_C|GetBP_HealthSystem_AC _asbp_player_with_anim))))
          (Variables|Default|SetHitting _returnvalue))))))

(fn ConstructionScript)