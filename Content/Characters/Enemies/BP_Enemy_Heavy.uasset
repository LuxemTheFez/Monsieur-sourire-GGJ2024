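; BP_Enemy_Heavy is a heavy enemy character Blueprint that specializes a parent enemy class.
; On BeginPlay it runs the parent logic, overrides maximum health and fills current health to match, then assigns the ABP_Heavy_Enemy animation Blueprint to the mesh.
; It also stores its Sphere component as HitSphere, while overlap and Tick events remain disabled and the construction script only calls the parent.
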(event EventBeginPlay
  (|CallParentFunction)
  (bind _output_get (Variables|Default|SetMaxHealth 2.0))
  (Variables|Default|SetCurrentHealth _output_get)
  (Class|SkeletalMeshComponent|SetAnimClass (Variables|Character|GetMesh) "/Game/Characters/Enemies/ABP_Heavy_Enemy.ABP_Heavy_Enemy_C")
  (Variables|Default|SetHitSphere (Variables|Default|GetSphere)))

(event Collision|EventActorBeginOverlap
  (params (OtherActor :type Actor%20Object%20Reference)))

(event EventTick
  (params (DeltaSeconds :type Float%20%28single-precision%29))
  (|CallParentFunction DeltaSeconds) ; This node is disabled and will not be called.\nDrag off pins to build functionality.
)

(fn ConstructionScript
  (|CallParentFunction))