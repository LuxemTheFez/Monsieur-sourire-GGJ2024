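; BP_Cacatapulte is an interactable catapult that players load with poop from their bucket and fire at a target.
; Holding interact unloads the bucket into the projectile's damage level up to 100, while a press with an empty bucket launches a loaded shot.
; One timeline swings the spoon, then reverses at a rearm-time rate before setting it armed again.
; An overlap box toggles the prompt widget, whose text Tick refreshes.
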(event OnComponentBeginOverlap(Box)
  (params (OverlappedComponent :type Primitive%20Component%20Object%20Reference) (OtherActor :type Actor%20Object%20Reference) (OtherComp :type Primitive%20Component%20Object%20Reference) (OtherBodyIndex :type Integer) (bFromSweep :type Boolean) (SweepResult :type Hit%20Result%20Structure%20%28by%20ref%29))
  (if (== OtherActor (Game|GetPlayerCharacter 0))
    (UserInterface|Viewport|AddtoViewport (Variables|Default|GetInteract%20Prompt) 0)))

(event OnComponentEndOverlap(Box)
  (params (OverlappedComponent :type Primitive%20Component%20Object%20Reference) (OtherActor :type Actor%20Object%20Reference) (OtherComp :type Primitive%20Component%20Object%20Reference) (OtherBodyIndex :type Integer))
  (if (== (Game|GetPlayerCharacter 0) OtherActor)
    (Widget|RemovefromParent (Variables|Default|GetInteract%20Prompt))))

(event Custom|LaunchPoop
  ;[1 1 1] Launch Poop
  (if (Variables|Default|GetisArmed?)
    (Variables|Default|SetPoop%20In%20Travel true)
    (Default|Move (Variables|Default|Getprojectile) (Variables|Default|GetpoopTarget))
    (Variables|Default|SetisArmed? false)))

(event Custom|Launch%20Spoon%20Anim
  ;[1 1 1] Spoon Animation
  (bind _spoon_track (Timeline|Rotate%20Spoon%20T PlayFromStart)
    (:Update
      (Transformation|SetRelativeRotation (Variables|Default|GetCacapulte_spoon) (Math|Rotator|MakeRotator (Math|Float|Lerp (Variables|Default|GetArmed%20Position) (Variables|Default|GetLaunched%20Position) _spoon_track) 0.0 0.0) false false))
    (:Finished
      (if (Variables|Default|Getis%20Reloading?)
        (Variables|Default|SetisArmed? true)
        (Variables|Default|Setis%20Reloading? false)
        (else
          (Components|Timeline|SetPlayRate (Variables|Default|GetRotate%20Spoon%20T) (/ 1.0 (Variables|Default|GetTime%20to%20arm%20%28s%29)))
          (Variables|Default|Setis%20Reloading? true)
          (Timeline|Rotate%20Spoon%20T Reverse))))))

(event Custom|Fill%20with%20poop
  (params (amount%20to%20add :type Integer))
  (Variables|Default|SetPoop%20In%20Travel false)
  (bind _poopy_percent (CallFunction|GetPoopyLevel))
  (CallFunction|SetPoopLevel (+ _poopy_percent amount%20to%20add)))

(event Custom|Set%20Poop%20Level
  (params (amount :type Integer))
  (Default|SetDamage (Variables|Default|Getprojectile) amount))

(event Collision|EventActorBeginOverlap
  (params (OtherActor :type Actor%20Object%20Reference)))

(event EventTick
  (params (DeltaSeconds :type Float%20%28single-precision%29))
  (CallFunction|GetInteractPrompt))

(event EventBeginPlay
  (bind _returnvalue (UserInterface|CreateWidget "/Game/Characters/W_Interact.W_Interact_C"))
  (Variables|Default|SetInteract%20Prompt _returnvalue)
  (Variables|Default|SetisArmed? true)
  (Variables|Default|Setis%20Reloading? false))

(fn ConstructionScript)

(fn GetPoopyLevel
  (return (Variables|/Game/Characters/BP_caca.BP_caca_C|GetPoopy%20Damage (Variables|Default|Getprojectile))))

(fn GetInteractPrompt
  (bind _interact_prompt (Variables|Default|GetInteract%20Prompt))
  (if (Variables|Default|GetisArmed?)
    (bind _usable_ (CallFunction|Usable))
    (if _usable_
      (CallFunction|GetPoopyLevel)
      (Default|SetText _interact_prompt "E to interact"))
    (else
      (Default|SetText _interact_prompt "Rearming catapult..."))))

(fn Usable
  (bind _poopy_percent (CallFunction|GetPoopyLevel))
  (return (or (<= _poopy_percent 0) (not (Variables|Default|GetPoop%20In%20Travel)))))

(fn Interact
  (params (Interactor :type Character%20Object%20Reference))
  (bind _asbp_test_character_lucas (Utilities|Casting|CastToBP_TestCharacter_Lucas Interactor))
  (bind _bucket_fillage (Default|GetBucketFillage _asbp_test_character_lucas))
  (if (<= _bucket_fillage 0)
    (bind _poopy_percent (CallFunction|GetPoopyLevel))
    (if (and (Variables|Default|GetisArmed?) (!= _poopy_percent 0))
      (CallFunction|LaunchPoop)
      (Components|Timeline|SetPlayRate (Variables|Default|GetRotate%20Spoon%20T) (/ 1.0 (Variables|Default|GetTime%20to%20launch%20%28s%29)))
      (CallFunction|LaunchSpoonAnim)
      (return true)
      (else
        (return false)))
    (else
      (return false))))

(fn InteractHold
  (params (Interactor :type Character%20Object%20Reference))
  (bind _asbp_test_character_lucas (Utilities|Casting|CastToBP_TestCharacter_Lucas Interactor)
    (:then
      (bind _poopy_percent (CallFunction|GetPoopyLevel))
      (if (or (>= _poopy_percent 100) (not (Variables|Default|GetisArmed?)))
        (return false)
        (else
          (bind _succeeded (Default|UnloadPoop _asbp_test_character_lucas))
          (if _succeeded
            (CallFunction|FillwithPoop 1)
            (return true)))))
    (:CastFailed
      (return false))))