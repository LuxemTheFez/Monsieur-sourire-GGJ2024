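; Health component for characters that tracks current health against a maximum, starting at full on BeginPlay.
; Tick accumulates time since the last hit, so TakeDamage only applies damage after a half-second invulnerability window, then resets that timer.
; Damage and Heal clamp health between zero and the maximum, and GetPercentage returns the remaining health as a percentage.
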(event EventBeginPlay
  (Variables|Default|SetcurentHealth (Variables|Default|GetmaxHealth)))

(event EventTick
  (params (DeltaSeconds :type Float%20%28single-precision%29))
  (Variables|Default|SetsecondSinceLastDmg (+ DeltaSeconds (Variables|Default|GetsecondSinceLastDmg))))

(fn TakeDamage
  (params (amount :type Integer))
  (if (>= (Variables|Default|GetsecondSinceLastDmg) 0.5)
    (Variables|Default|SetsecondSinceLastDmg 0.0)
    (bind _output_get (Variables|Default|SetcurentHealth (- (Variables|Default|GetcurentHealth) amount)))
    (if (<= _output_get 0)
      (Variables|Default|SetcurentHealth 0))))

(fn Heal
  (params (amount :type Integer))
  (bind _maxhealth (Variables|Default|GetmaxHealth))
  (bind _output_get (Variables|Default|SetcurentHealth (+ (Variables|Default|GetcurentHealth) amount)))
  (if (>= _output_get _maxhealth)
    (Variables|Default|SetcurentHealth _maxhealth)))

(fn GetPercentage
  (return (* (/ (Math|Conversions|ToFloat(Integer) (Variables|Default|GetcurentHealth)) (Math|Conversions|ToFloat(Integer) (Variables|Default|GetmaxHealth))) 1e+02)))