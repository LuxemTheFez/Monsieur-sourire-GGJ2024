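; Actor that flies in an arc from its current location to a target point over TravelTime, once its Move event is called.
; Move stores start and target, then Tick advances elapsed time and feeds a clamped alpha to MoveToTarget.
; MoveToTarget follows a cubic Bézier built from nested lerps, with GetRefs placing two control points along the line, raised by LaunchHeight.
; Move never resets the timer, and DestroyActor is unconnected.
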(event Custom|Move
  (params (Target :type Vector))
  (Variables|Default|SetTarget Target)
  (Variables|Default|SetBaseLocation (Transformation|GetActorLocation))
  (Variables|Default|SetHas%20Target true))

(event EventBeginPlay)

(event EventTick
  (params (DeltaSeconds :type Float%20%28single-precision%29))
  (if (and (Variables|Default|GetHas%20Target) (< (Variables|Default|GetTime%20Since%20Launched) (Variables|Default|GetTravel%20Time)))
    (bind _output_get (Variables|Default|SetTime%20Since%20Launched (+ DeltaSeconds (Variables|Default|GetTime%20Since%20Launched))))
    (CallFunction|MovetoTarget (Math|Float|Min(Float) (/ _output_get (Variables|Default|GetTravel%20Time)) 1.0))))

(event Collision|EventActorBeginOverlap
  (params (OtherActor :type Actor%20Object%20Reference)))

(fn ConstructionScript)

(fn MovetoTarget
  (params (Alpha :type Float%20%28double-precision%29))
  (bind _target (Variables|Default|GetTarget))
  (bind _baselocation (Variables|Default|GetBaseLocation))
  (bind (_ref1 _ref2) (CallFunction|GetRefs _baselocation _target))
  (Transformation|SetActorLocation (Math|Vector|Lerp(Vector) (Math|Vector|Lerp(Vector) (Math|Vector|Lerp(Vector) _baselocation _ref1 Alpha) (Math|Vector|Lerp(Vector) _ref1 _ref2 Alpha) Alpha) (Math|Vector|Lerp(Vector) (Math|Vector|Lerp(Vector) _ref1 _ref2 Alpha) (Math|Vector|Lerp(Vector) _ref2 _target Alpha) Alpha) Alpha) false false))

(fn GetRefs
  (params (Start :type Vector) (End :type Vector))
  (bind _returnvalue (- End Start))
  (bind _launch_height_ (Variables|Default|GetLaunch%20Height%20))
  (bind _returnvalue_2 (Math|Vector|MakeVector 0.0 0.0 _launch_height_))
  (bind _returnvalue_3 (/ _returnvalue 9.0))
  (return (+ Start (* _returnvalue_3 3.5) _returnvalue_2) (+ Start (* _returnvalue_3 5.5) _returnvalue_2)))