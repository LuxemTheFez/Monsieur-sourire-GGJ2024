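; BP_JackBox is a jack-in-the-box item that winds up while a BP_LeoTest stands in its trigger and entertains the boss when it pops.
; Tick accumulates time in the zone to spin the crank, rewinding it at RewindSpeed when the zone is empty.
; At SecToOpen it opens once: the crank detaches and flies off with physics, then after a short delay Jack appears, animates and EntertainBoss is called.
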(event OnComponentEndOverlap(Box1)
  (params (OverlappedComponent :type Primitive%20Component%20Object%20Reference) (OtherActor :type Actor%20Object%20Reference) (OtherComp :type Primitive%20Component%20Object%20Reference) (OtherBodyIndex :type Integer))
  (Utilities|Casting|CastToBP_LeoTest OtherActor)
  (Variables|Default|SetplayerInZone false))

(event OnComponentBeginOverlap(Box1)
  (params (OverlappedComponent :type Primitive%20Component%20Object%20Reference) (OtherActor :type Actor%20Object%20Reference) (OtherComp :type Primitive%20Component%20Object%20Reference) (OtherBodyIndex :type Integer) (bFromSweep :type Boolean) (SweepResult :type Hit%20Result%20Structure%20%28by%20ref%29))
  (Utilities|Casting|CastToBP_LeoTest OtherActor)
  (Variables|Default|SetplayerInZone true))

(event EventBeginPlay
  (Variables|Default|SetfunAdded 0.45)
  (Components|Animation|PlayAnimation (Variables|Default|GetBox) "/Game/Props/Jack_in_the_box/Jack_box_closed_Anim.Jack_box_closed_Anim" false))

(event EventTick
  (params (DeltaSeconds :type Float%20%28single-precision%29))
  (bind _sectoopen (Variables|Default|GetsecToOpen))
  (bind _jack (Variables|Default|GetJack))
  (bind _jack_manivelle (Variables|Default|GetJack_manivelle))
  (if (Variables|Default|GetplayerInZone)
    (bind _output_get (Variables|Default|SettimeAlive (+ DeltaSeconds (Variables|Default|GettimeAlive))))
    (if (and (< _output_get _sectoopen) (not (Variables|Default|Getopened))) :!label _label
      (Transformation|SetWorldRotation (Variables|Default|GetOrigin) (Math|Rotator|MakeRotator (* _output_get 3.6e+02) 0.0 0.0) false false)
      (elif (and (>= _output_get _sectoopen) (not (Variables|Default|Getopened)))
        (Variables|Default|Setopened true)
        (Components|Animation|PlayAnimation (Variables|Default|GetBox) "/Game/Props/Jack_in_the_box/Jack_Box_Anims_Anim.Jack_Box_Anims_Anim" false)
        (Transformation|DetachFromComponent (Variables|Default|GetOrigin) "KeepWorld" "KeepWorld" "KeepWorld" true)
        (Physics|SetSimulatePhysics _jack_manivelle true)
        (Physics|AddForce _jack_manivelle "-100000.000000,0.000000,200000.000000" "None" true)
        (Utilities|FlowControl|Delay 0.5)
        (Transformation|SetWorldScale3D _jack "1.000000,1.000000,1.000000")
        (Components|Animation|PlayAnimation _jack "/Game/Props/Jack_in_the_box/Jack_Chara_Anim.Jack_Chara_Anim" false)
        (CallFunction|EntertainBoss)))
    (elif (> (Variables|Default|GettimeAlive) 0.0)
      (Variables|Default|SettimeAlive (Math|Float|Max(Float) (- (Variables|Default|GettimeAlive) (* DeltaSeconds (Variables|Default|GetrewindSpeed))) 0.0))
      (goto _label))))

(fn ConstructionScript)