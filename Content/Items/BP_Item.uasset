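; BP_Item is a base item that players grab on overlap and bring to the stage to entertain the Boss.
; Touching a BP_StageCollider marks it on stage and tells the owning player to drop it.
; Dropped detaches it, moves it to the first "ItemHolder" actor with random yaw, and switches collision from grabbing to interaction.
; Later overlaps call the empty OnInteractCollision hook, and helper functions report fun to the Boss by item class.
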(event Custom|Dropped
  (CallFunction|CanInteract)
  (Transformation|DetachFromActor "KeepWorld" "KeepWorld" "KeepWorld")
  (bind _outactors (Actor|GetAllActorswithTag "ItemHolder"))
  (Transformation|SetActorTransform (Math|Transform|MakeTransform (Transformation|GetActorLocation (Utilities|Array|Get(acopy) _outactors)) (Math|Rotator|MakeRotator 0.0 0.0 (* (Math|Random|RandomFloat) 3.6e+02)) "1.000000,1.000000,1.000000") false true)
  (Variables|Default|SetisGrabbed false))

(event EventBeginPlay)

(event Collision|EventActorBeginOverlap
  (params (OtherActor :type Actor%20Object%20Reference))
  (if (and (Variables|Default|GetisOnStage) (not (Variables|Default|GetisGrabbed)))
    (CallFunction|OnInteractCollision OtherActor)
    (elif (not (Variables|Default|GetisOnStage))
      (Utilities|Casting|CastToBP_StageCollider OtherActor
        (:then
          (Variables|Default|SetisOnStage true)
          (bind _asbp_player_with_anim (Utilities|Casting|CastToBP_PlayerWithAnim (Variables|Default|GetPlayerOwner)))
          (Default|Drop _asbp_player_with_anim))
        (:CastFailed
          (if (not (Variables|Default|GetisGrabbed))
            (bind _asbp_player_with_anim_2 (Utilities|Casting|CastToBP_PlayerWithAnim OtherActor))
            (bind _isgrabbed (Default|Grab _asbp_player_with_anim_2 self))
            (Variables|Default|SetisGrabbed _isgrabbed)
            (Variables|Default|SetPlayerOwner _asbp_player_with_anim_2)))))))

(event EventTick
  (params (DeltaSeconds :type Float%20%28single-precision%29)))

(fn ConstructionScript)

(fn EntertainBoss
  (Default|Entertain (Variables|Default|GetBoss) (Variables|Default|GetfunAdded) (Utilities|GetClass self)))

(fn EntertainOverTimeBoss
  (params (deltaTime :type Float%20%28double-precision%29))
  (Default|EntertainOverTime (Variables|Default|GetBoss) (* deltaTime (Variables|Default|GetfunAdded)) (Utilities|GetClass self)))

(fn ConsiderEntertainBoss
  (Default|ConsiderEntertainer (Variables|Default|GetBoss) (Utilities|GetClass self)))

(fn CanInteract
  (Collision|SetCollisionEnabled (Variables|Default|GetitemGrabCollider) "NoCollision")
  (Collision|SetCollisionProfileName (Variables|Default|GetitemInteractCollider) "OverlapAllDynamic" false :!class /Script/Engine.PrimitiveComponent))

(fn OnInteractCollision
  (params (Other%20Actor :type Actor%20Object%20Reference)))