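; Whoopee cushion item that starts farting when a BP_LeoTest actor overlaps it and destroys itself when that overlap ends.
; Overlap activates the Niagara effect and sets a farting flag.
; While farting, Tick rapidly wobbles the FarterOrigin yaw with a sine wave around its starting rotation and calls EntertainOverTimeBoss, with the fun amount set at BeginPlay.
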(event Custom|OnComponentBeginOverlap_Event
  (params (OverlappedComponent :type Primitive%20Component%20Object%20Reference) (OtherActor :type Actor%20Object%20Reference) (OtherComp :type Primitive%20Component%20Object%20Reference) (OtherBodyIndex :type Integer) (bFromSweep :type Boolean) (SweepResult :type Hit%20Result%20Structure%20%28by%20ref%29))
  (Utilities|Casting|CastToBP_LeoTest OtherActor)
  (Variables|Default|SetisFarting true)
  (Components|Activation|Activate (Variables|Default|GetNS_Whooping_Cushion) false))

(event Custom|OnComponentEndOverlap_Event
  (params (OverlappedComponent :type Primitive%20Component%20Object%20Reference) (OtherActor :type Actor%20Object%20Reference) (OtherComp :type Primitive%20Component%20Object%20Reference) (OtherBodyIndex :type Integer))
  (Utilities|Casting|CastToBP_LeoTest OtherActor)
  (Actor|DestroyActor))

(event EventBeginPlay
  (Variables|Default|SetfunAdded 0.2)
  (Variables|Default|SetbaseRotation (Transformation|GetWorldRotation (Variables|Default|GetFarterOrigin)))
  (Collision|AssignOnComponentBeginOverlap (Variables|Default|GetWhoopingCushion) (delegate Custom|OnComponentBeginOverlap_Event))
  (Collision|AssignOnComponentEndOverlap (Variables|Default|GetWhoopingCushion) (delegate Custom|OnComponentEndOverlap_Event)))

(event EventTick
  (params (DeltaSeconds :type Float%20%28single-precision%29))
  (bind _baserotation (Variables|Default|GetbaseRotation))
  (bind _output_get (Variables|Default|SettimeAlive (+ DeltaSeconds (Variables|Default|GettimeAlive))))
  (if (Variables|Default|GetisFarting)
    (Transformation|SetWorldRotation (Variables|Default|GetFarterOrigin) (Math|Rotator|MakeRotator (.roll _baserotation) (.pitch _baserotation) (+ (* (Math|Trig|Sin(Radians) (* _output_get 5e+01)) 3e+01) (.yaw _baserotation))) false false)
    (CallFunction|EntertainOverTimeBoss DeltaSeconds)))

(fn ConstructionScript)