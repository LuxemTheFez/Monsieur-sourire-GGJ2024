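; BP_Poop_Container is an interactable item that lets the player fill a bucket.
; It creates a W_Interact prompt on BeginPlay and shows or removes it as the player character enters or leaves its Box trigger.
; InteractHold calls FillBucket on a BP_PlayerWithAnim interactor and reports success, while plain Interact always returns false, so only a hold interaction fills the bucket.
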(event OnComponentBeginOverlap(Box)
  (params (OverlappedComponent :type Primitive%20Component%20Object%20Reference) (OtherActor :type Actor%20Object%20Reference) (OtherComp :type Primitive%20Component%20Object%20Reference) (OtherBodyIndex :type Integer) (bFromSweep :type Boolean) (SweepResult :type Hit%20Result%20Structure%20%28by%20ref%29))
  (if (== OtherActor (Game|GetPlayerCharacter 0))
    (UserInterface|Viewport|AddtoViewport (Variables|Default|GetInteractPrompt) 0)))

(event OnComponentEndOverlap(Box)
  (params (OverlappedComponent :type Primitive%20Component%20Object%20Reference) (OtherActor :type Actor%20Object%20Reference) (OtherComp :type Primitive%20Component%20Object%20Reference) (OtherBodyIndex :type Integer))
  (if (== (Game|GetPlayerCharacter 0) OtherActor)
    (Widget|RemovefromParent (Variables|Default|GetInteractPrompt))))

(event EventBeginPlay
  (bind _returnvalue (UserInterface|CreateWidget "/Game/Characters/W_Interact.W_Interact_C"))
  (bind _output_get (Variables|Default|SetInteractPrompt _returnvalue))
  (Default|SetText _output_get "E to fill your bucket"))

(fn ConstructionScript)

(fn Interact
  (params (Interactor :type Character%20Object%20Reference))
  (return false))

(fn InteractHold
  (params (Interactor :type Character%20Object%20Reference))
  (bind _asbp_player_with_anim (Utilities|Casting|CastToBP_PlayerWithAnim Interactor)
    (:then
      (Default|FillBucket _asbp_player_with_anim)
      (return true))
    (:CastFailed
      (return false))))